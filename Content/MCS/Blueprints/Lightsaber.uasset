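; Lightsaber weapon for MCS characters, with timeline-driven blade extend and retract, hum and impact effects, and dynamic color.
; While hit detection is enabled, a Tick gate runs box traces between current and stored blade socket positions, on server, client or both.
; A Visibility trace catches blade clashes before a weapon-channel fallback can hit players.
; Hits notify the owning character, and blade-on-blade contact disables detection and records the other weapon's velocities.
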(event `Initialize`
  ;[1 1 1] Initialize and set references
  (set `self.DefaultCollision` (`PrimitiveComponent.GetCollisionEnabled` (`self.Blade`)))
  (set `self.IsWeaponDrawn?` false))

(event `GrabHilt`
  ;[1 1 1] HACK to grab the hilt (just makes it visible)
  (`SceneComponent.SetVisibility` (`self.Hilt`) true true))

(event `BladeHitBlade`
  (params (ImpactPoint :type "Vector Structure") (CausedBy :type "/Game/MCS/Blueprints/MCSCharacter Object Reference"))
  ;[1 1 1] Spawn a particle effect at the point of impact
  (`GameplayStatics.PlaySoundAtLocation` "/Game/MCS/Sounds/Saber/SaberHits_Cue.SaberHits_Cue" ImpactPoint)
  (`GameplayStatics.SpawnEmitterAtLocation` "/Game/MCS/ParticleFX/P_SaberImpact.P_SaberImpact" ImpactPoint))

(event `UpdateSaberColor`
  (params (Color :type "LinearColor Structure"))
  (bind _bladematerial (`self.BladeMaterial`))
  ;[1 1 1] Lightsaber blade color
  (bind _output_get (set `self.SaberColor` Color))
  (`MaterialInstanceDynamic.SetVectorParameterValue` _bladematerial "EmissiveColor" _output_get)
  (`MaterialInstanceDynamic.SetVectorParameterValue` _bladematerial "EmissiveStrength" (struct :`R` 50.0 :`G` 50.0 :`B` 50.0 :`A` 1.0))
  (`LightComponent.SetLightColor` (`self.BladeLight`) (`self.SaberColor`) true))

(event `DrawSheathWeapon`
  (bind _saberhum (`self.SaberHum`))
  ;[1 1 1] Turn lightsaber ON/OFF.  Enable/Disable collision respectively.
  (if (`self.IsWeaponDrawn?`)
    (`SceneComponent.SetVisibility` (`self.Hilt`) true true)
    (`GameplayStatics.PlaySoundAtLocation` "/Game/MCS/Sounds/Saber/saberon_Cue.SaberOn_Cue" (`self.K2_GetActorLocation`))
    (`AudioComponent.SetVolumeMultiplier` _saberhum 1.0)
    (`AudioComponent.Play` _saberhum 0.0)
    (bind (_direction _bladezlength) (`Timeline|BladeExtendTime` :!via `PlayFromStart`)
      (:`Update`
        (`SceneComponent.SetWorldScale3D` (`self.Blade`) (`KismetMathLibrary.MakeVector` 1.0 1.0 _bladezlength))
        (`LightComponent.SetIntensity` (`self.BladeLight`) (* _bladezlength (`self.DefaultLightIntesity`)))
        (set `self.IsWeaponDrawn?` true)
        (`PrimitiveComponent.SetCollisionEnabled` (`self.Blade`) "QueryAndPhysics")))
    (else
      (`GameplayStatics.PlaySoundAtLocation` "/Game/MCS/Sounds/Saber/saberoff_Cue.SaberOff_Cue" (`self.K2_GetActorLocation`))
      (bind (_direction_2 _bladezlength_2) (`Timeline|BladeContractTime` :!via `PlayFromStart`)
        (:`Update`
          (`SceneComponent.SetWorldScale3D` (`self.Blade`) (`KismetMathLibrary.MakeVector` 1.0 1.0 _bladezlength_2))
          (`LightComponent.SetIntensity` (`self.BladeLight`) (* _bladezlength_2 (`self.DefaultLightIntesity`)))
          (set `self.IsWeaponDrawn?` false)
          (`PrimitiveComponent.SetCollisionEnabled` (`self.Blade`) "NoCollision"))
        (:`Finished`
          (`AudioComponent.Stop` (`self.SaberHum`)))))))

(event `ToggleTraceVisibility`
  ;[1 0.8453 0.2404] DEBUG: Toggle trace lines / hit information.
  (if (`|EnumEquality` "None" (`self.DebugDrawType`))
    (bind _output_get (set `self.DebugDrawType` "ForDuration"))
    (`KismetSystemLibrary.PrintString` (`KismetStringLibrary.Concat_StrStr` "Trace Lines:  " (`|GetEnumeratorNameAsString` _output_get)))
    (else
      (bind _output_get_2 (set `self.DebugDrawType` "None"))
      (`KismetSystemLibrary.PrintString` (`KismetStringLibrary.Concat_StrStr` "Trace Lines:  " (`|GetEnumeratorNameAsString` _output_get_2))))))

(event `ToggleHitInfo`
  ;[1 0.8453 0.2404] DEBUG: Toggle trace lines / hit information.
  (bind _output_get (set `self.bDisplayHitInfo` (not (`self.bDisplayHitInfo`))))
  (if _output_get
    (`KismetSystemLibrary.PrintString` "Hit info is ON")
    (else
      (`KismetSystemLibrary.PrintString` "Hit info is OFF"))))

(event `self.ReceiveTick`
  (params (DeltaSeconds :type "Float (single-precision)"))
  (bind (_bblockinghit _binitialoverlap _time _location _impactpoint _normal _impactnormal _physmat _hitactor _hitcomponent _hitbonename) (`GameplayStatics.BreakHitResult` (`self.WeaponHitResult`)))
  (bind _returnvalue (`GameplayStatics.GetObjectClass` _hitactor))
  ;[1 0.38 0.38] Enables/Disables Hit Detection traces for this weapon
  (`/Engine/EditorBlueprintResources/StandardMacros.Gate` true :!label _label
    (:`Exit`
      ;;[1 1 1] Trace for blade hitting blade collisions ONLY.  The player mesh is setup to not respond to trace hits on this channel (visibility) - thus the player mesh will never be hit by this trace.
      (bind (_hitresult _weaponhit_) (`self.WeaponTrace` (`self.DefaultTraceChannel`)))
      (set `self.WeaponHitResult` _hitresult)
      (if _weaponhit_
        (if (`KismetMathLibrary.ClassIsChildOf` _returnvalue "Lightsaber_C") :!label _label_2
          (if (`self.bDisplayHitInfo`)
            (`/Game/MCS/Blueprints/Macros/Utilities.PrintHitInfo` (struct :`G` 1.0 :`B` 0.027451 :`A` 1.0) (`self.WeaponHitResult`) 2.0))
          (bind _asmcscharacter (`self.GetCharacter`))
          (`/Game/MCS/Blueprints/MCSCharacter.OnBladeHitBlade` _asmcscharacter (`self.WeaponHitResult`) _asmcscharacter)
          (elif (and (`KismetMathLibrary.ClassIsChildOf` _returnvalue "/Game/MCS/Blueprints/MCSCharacter.MCSCharacter_C") (not (`KismetArrayLibrary.Array_Contains` (`self.ExcludedBones`) _hitbonename)))
            (if (`self.bDisplayHitInfo`)
              (`/Game/MCS/Blueprints/Macros/Utilities.PrintHitInfo` (struct :`G` 0.347601 :`B` 1.0 :`A` 1.0) (`self.WeaponHitResult`) 2.0))
            (bind _asmcscharacter_2 (`self.GetCharacter`))
            (`/Game/MCS/Blueprints/MCSCharacter.OnBladeHitPlayer` _asmcscharacter_2 (`self.WeaponHitResult`) _asmcscharacter_2)))
        (else
          ;;[1 1 1] A few ticks after the visibility trace. This trace responds to BOTH the visibility channel AND the weapons channel.  The player mesh is setup to respond only to the weapon channel trace. This trace can hit both the other players weapon and the other player.
          (bind (_hitresult_2 _weaponhit__2) (`self.WeaponTrace` "TraceTypeQuery3"))
          (set `self.WeaponHitResult` _hitresult_2)
          (if _weaponhit__2
            (goto _label_2)))))))

(event `EnableHitDetection`
  (params (Enable :type Boolean))
  (bind _returnvalue (`self.GetParentActor`))
  (bind (_asmcscharacter _bsuccess) (cast `/Game/MCS/Blueprints/MCSCharacter` _returnvalue :!pure true))
  ;[1 0.38 0.38] Enables/Disables Hit Detection traces for this weapon
  (bind _output_get (set `self.hitDetectionEnabled` Enable))
  (`self.SetCollision` _output_get)
  (switch `/Game/MCS/Blueprints/Enums/MCSHitDetectionType` (`self.HitDetectionType`)
    (:`NewEnumerator0`
      ;;[1 0 0] Trace runs on server only
      (`/Engine/EditorBlueprintResources/ActorMacros.Switch Has Authority`
        (:`Authority`
          _)))
    (:`NewEnumerator1`
      ;;[1 0 0] Trace runs on clients only
      (`/Engine/EditorBlueprintResources/ActorMacros.Switch Has Authority`
        (:`Remote`
          _)))
    (:`NewEnumerator2`
      _))
  (if _bsuccess
    (`KismetArrayLibrary.Array_Set` (`self.ActorsToIgnore`) 0 _asmcscharacter true)
    (if (and (`self.hitDetectionEnabled`) (`self.IsWeaponDrawn?`))
      (set `self.DebugDrawType` (`self.DebugDrawType`))
      (`self.ResetWeaponSockets`)
      (goto _label :!via `Open`)
      (else
        (goto _label :!via `Close`)))
    (else
      (`/Game/MCS/Blueprints/Macros/Utilities.InvalidCastInfo` _returnvalue))))

(fn `PrintPhysicsInfo`
  (`KismetSystemLibrary.PrintString` (`KismetSystemLibrary.GetDisplayName` self))
  (`KismetSystemLibrary.PrintString` (`KismetStringLibrary.Concat_StrStr` "Linear:  " (`KismetStringLibrary.Conv_VectorToString` (`self.LinearVelocity`)) "      " "Angular:  " (`KismetStringLibrary.Conv_VectorToString` (`self.AngularVelocity`)) "      " "Linear at Point:  " (`KismetStringLibrary.Conv_VectorToString` (`self.LinearVelocityAtPoint`)))))

(fn `SetCollision`
  (params (Enable :type Boolean))
  (if (`self.NoCollisionWhenIdle`)
    (if Enable
      (`PrimitiveComponent.SetCollisionEnabled` (`self.Hilt`) (`self.DefaultCollision`))
      (`PrimitiveComponent.SetCollisionEnabled` (`self.Blade`) (`self.DefaultCollision`))
      (else
        (`PrimitiveComponent.SetCollisionEnabled` (`self.Hilt`) "NoCollision")
        (`PrimitiveComponent.SetCollisionEnabled` (`self.Blade`) "NoCollision")))))

(fn `UserConstructionScript`
  (set `self.DefaultLightIntesity` (`LightComponentBase.Intensity` (`self.BladeLight`)))
  (if (not (`self.IsWeaponDrawn?`))
    (`LightComponent.SetIntensity` (`self.BladeLight`) 0.0)
    (`SceneComponent.SetWorldScale3D` (`self.Blade`) (`KismetMathLibrary.MakeVector` 1.0 1.0))
    (`SceneComponent.SetVisibility` (`self.Hilt`) false true))
  (bind _returnvalue (`PrimitiveComponent.CreateDynamicMaterialInstance` (`self.Blade`) 0 "/Game/MCS/Materials/Glow_MI.Glow_MI"))
  (bind _output_get (set `self.BladeMaterial` _returnvalue))
  (`MaterialInstanceDynamic.SetVectorParameterValue` _output_get "EmissiveColor" (`self.SaberColor`))
  (`LightComponent.SetLightColor` (`self.BladeLight`) (`self.SaberColor`) true))