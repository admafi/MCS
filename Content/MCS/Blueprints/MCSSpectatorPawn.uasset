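; MCS spectator pawn that can frame a player character on spawn and receives a player profile.
; On BeginPlay, if LookAtPlayer is set, it moves to an offset from the first MCSCharacter at fixed height and turns its controller toward it once.
; OnSendPlayerProfile stores the profile and passes it with player controller 0 to SendPlayerProfile, which is empty.
; The ServerUpdatePlayerProfile call is disconnected and never runs.
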(event `self.ReceiveBeginPlay`
  (bind _returnvalue (`self.GetController`))
  (if (`self.bLookAtPlayer`)
    (bind _outactors (`GameplayStatics.GetAllActorsOfClass` "/Game/MCS/Blueprints/MCSCharacter.MCSCharacter_C"))
    (bind _output (`|GetArrayItem` _outactors))
    (`/Engine/EditorBlueprintResources/StandardMacros.IsValid` _output
      (:`Is Valid`
        (`/Engine/EditorBlueprintResources/StandardMacros.IsValid` _returnvalue
          (:`Is Valid`
            (bind _returnvalue_2 (`self.K2_GetActorLocation` _output))
            (`self.K2_SetActorLocation` (`KismetMathLibrary.MakeVector` (+ (.x _returnvalue_2) 300.0) (- (.y _returnvalue_2) 400.0) 600.0))
            (`Controller.SetControlRotation` _returnvalue (`KismetMathLibrary.FindLookAtRotation` (`self.K2_GetActorLocation`) _returnvalue_2))))))))

(event `SendPlayerProfile`
  (params (playerProfile :type "/Game/MCS/Blueprints/AllLevels/MCSPlayerInfo Structure") (playerController :type "PlayerController Object Reference")))

(event `OnSendPlayerProfile`
  (params (playerProfile :type "/Game/MCS/Blueprints/AllLevels/MCSPlayerInfo Structure"))
  (bind _output_get (set `self.PlayerProfile` playerProfile))
  (`self.SendPlayerProfile` _output_get (`GameplayStatics.GetPlayerController` 0)))

(fn `UserConstructionScript`)