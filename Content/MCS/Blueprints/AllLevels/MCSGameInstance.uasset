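; Game instance that manages front-end menus, online sessions and the saved player profile.
; The profile check loads an existing save and opens the main menu, or opens options when none exists.
; Events create and show UI widgets and wrap session create, join and destroy, with timed server and error popups.
; Session, network and travel failures route to DisplayErrorMessage, which is empty, as are the error-to-string conversions; the lobby level name is unset.
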(event `SavedProfileCheck`
  ;[1 1 1] Check if the players profile has already been saved
  (bind _returnvalue (`GameplayStatics.DoesSaveGameExist` (`self.PlayerProfileSave`)))
  (if _returnvalue
    (`self.LoadProfile`)
    (`self.ShowMainMenu`)
    (set `self.SaveGameExists?` true)
    (else
      (`self.ShowOptionsMenu`)
      (set `PlayerController.bShowMouseCursor` true (`GameplayStatics.GetPlayerController` 0))
      (set `self.SaveGameExists?` false))))

(event `ShowMainMenu`
  (bind _returnvalue (`GameplayStatics.GetPlayerController` 0))
  ;[0 0.7294 1] Show main menu and enable the mouse cursor
  (`/Engine/EditorBlueprintResources/StandardMacros.IsValid` (`self.mainMenu`)
    (:`Is Valid`
      _)
    (:`Is Not Valid`
      (bind _returnvalue_2 (`|CreateWidget` "/Game/MCS/UI/MainMenu/MainMenu.MainMenu_C" _returnvalue))
      (set `self.mainMenu` _returnvalue_2)))
  (`UserWidget.AddToViewport` (`self.mainMenu`) 0)
  (set `PlayerController.bShowMouseCursor` true _returnvalue)
  (`WidgetBlueprintLibrary.SetInputMode_UIOnlyEx` _returnvalue (`self.mainMenu`)))

(event `self.HandleNetworkError`
  (params (FailureType :type "ENetworkFailure Enum" :default "NetDriverAlreadyExists") (bIsServer :type Boolean))
  ;[1 0.38 0.38] Network and travel failure error handling
  (if bIsServer
    _
    (else
      _))
  (`self.DisplayErrorMessage` (`self.NetErrorToString` FailureType)))

(event `LaunchLobby`
  (params (maxPlayers :type Integer) (`enableLAN?` :type Boolean) (serverName :type Name))
  ;[0 1 0.2708] Launch the server lobby and create session
  (set `self.maxPlayers` maxPlayers)
  (set `self.enableLAN` `enableLAN?`)
  (set `self.serverName` serverName)
  (`self.ShowLoadingScreen`)
  (`CreateSessionCallbackProxy.CreateSession` (`GameplayStatics.GetPlayerController` 0) (`self.maxPlayers`) (`self.enableLAN`)
    (:`OnSuccess`
      (`GameplayStatics.OpenLevel` "None"))
    (:`OnFailure`
      (`self.DisplayErrorMessage` "FAILED TO CREATE SESSION"))))

(event `self.HandleTravelError`
  (params (FailureType :type "ETravelFailure Enum" :default "NoLevel"))
  ;[1 0.38 0.38] Network and travel failure error handling
  (`self.DisplayErrorMessage` (`self.TravelErrorToString` FailureType)))

(event `ShowServerMenu`
  ;[0 0.7294 1] Show server menu (search for host servers or add IP)
  (bind _returnvalue (`|CreateWidget` "/Game/MCS/UI/MainMenu/ServerMenu.ServerMenu_C" (`GameplayStatics.GetPlayerController` 0)))
  (bind _output_get (set `self.serverMenu` _returnvalue))
  (`UserWidget.AddToViewport` _output_get 0))

(event `JoinServer`
  (params (SessionToJoin :type "BlueprintSessionResult Structure"))
  ;[0 1 0.2708] Join server.  Called from server menu.
  (`self.ShowLoadingScreen`)
  (`JoinSessionCallbackProxy.JoinSession` (`GameplayStatics.GetPlayerController` 0) SessionToJoin
    (:`OnFailure`
      (`self.DisplayErrorMessage` "FAILED TO JOIN SESSION"))))

(event `ShowOptionsMenu`
  ;[0 0.7294 1] Show options menu
  (`/Engine/EditorBlueprintResources/StandardMacros.IsValid` (`self.optionsMenu`)
    (:`Is Valid`
      _)
    (:`Is Not Valid`
      (bind _returnvalue (`|CreateWidget` "/Game/MCS/UI/MainMenu/PlayerOptionsMenu.PlayerOptionsMenu_C" (`GameplayStatics.GetPlayerController` 0)))
      (set `self.optionsMenu` _returnvalue)))
  (`UserWidget.AddToViewport` (`self.optionsMenu`) 0))

(event `DestroySessionCaller`
  (params (playerController :type "PlayerController Object Reference"))
  ;[0 1 0.2708] Destroy session
  (`DestroySessionCallbackProxy.DestroySession` playerController
    (:`OnFailure`
      (`self.DisplayErrorMessage` "FAILED TO DESTROY SESSION"))))

(event `ShowLoadingScreen`
  ;[0 0.7294 1] Show loading screen
  (`/Engine/EditorBlueprintResources/StandardMacros.IsValid` (`self.loadingScreen`)
    (:`Is Valid`
      _)
    (:`Is Not Valid`
      (bind _returnvalue (`|CreateWidget` "/Game/MCS/UI/AllLevels/LoadingScreen.LoadingScreen_C" (`GameplayStatics.GetPlayerController` 0)))
      (set `self.loadingScreen` _returnvalue)))
  (`UserWidget.AddToViewport` (`self.loadingScreen`) 0))

(event `ShowServerMessage`
  (params (message :type Text))
  (bind _servermessage (`self.serverMessage`))
  ;[0 0.7294 1] Show server messages
  (set `self.serverMessageText` message)
  (`/Engine/EditorBlueprintResources/StandardMacros.IsValid` (`self.serverMessage`)
    (:`Is Valid`
      _)
    (:`Is Not Valid`
      (bind _returnvalue (`|CreateWidget` "/Game/MCS/UI/AllLevels/ServerMessage.ServerMessage_C" (`GameplayStatics.GetPlayerController` 0)))
      (set `self.serverMessage` _returnvalue)))
  (`/Game/MCS/UI/AllLevels/ServerMessage.SetMessage` _servermessage (`self.serverMessageText`))
  (if (not (`Widget.IsInViewport` _servermessage))
    (`UserWidget.AddToViewport` (`self.serverMessage`) 0)
    (`KismetSystemLibrary.RetriggerableDelay` (`self.messageDuration`))
    (`Widget.RemoveFromParent` (`self.serverMessage`))))

(event `ShowErrorMessage`
  (params (ErrorMessage :type Text))
  (bind _errormessage (`self.errorMessage`))
  ;[0 0.7294 1] Error Messages
  (set `self.errorMessageText` ErrorMessage)
  (`/Engine/EditorBlueprintResources/StandardMacros.IsValid` (`self.errorMessage`)
    (:`Is Valid`
      _)
    (:`Is Not Valid`
      (bind _returnvalue (`|CreateWidget` "/Game/MCS/UI/AllLevels/ErrorMessage.ErrorMessage_C" (`GameplayStatics.GetPlayerController` 0)))
      (set `self.errorMessage` _returnvalue)))
  (`/Game/MCS/UI/AllLevels/ErrorMessage.SetMessage` _errormessage (`self.errorMessageText`))
  (`UserWidget.AddToViewport` _errormessage 0)
  (`KismetSystemLibrary.RetriggerableDelay` (`self.messageDuration`))
  (`Widget.RemoveFromParent` (`self.errorMessage`)))

(fn `GetPlayerProfile`
  (returns (playerProfile :type "/Game/MCS/Blueprints/AllLevels/MCSPlayerInfo Structure"))
  (bind _playersavegameref (`self.playerSaveGameRef`))
  (`/Engine/EditorBlueprintResources/StandardMacros.IsValid` _playersavegameref
    (:`Is Valid`
      (return (`/Game/MCS/Blueprints/AllLevels/MCSPlayerSaveGame.PlayerProfile` _playersavegameref)))
    (:`Is Not Valid`
      (`self.ShowErrorMessage` "Unable to get player profile"))))

(fn `LoadProfile`
  (bind _returnvalue (`GameplayStatics.LoadGameFromSlot` (`self.PlayerProfileSave`)))
  (bind _asmcsplayer_save_game (cast `/Game/MCS/Blueprints/AllLevels/MCSPlayerSaveGame` _returnvalue))
  (set `self.playerSaveGameRef` _asmcsplayer_save_game))

(fn `NetErrorToString`
  (params (failureType :type "ENetworkFailure Enum"))
  (returns (outputString :type String))
  (return ""))

(fn `SaveProfile`
  (`/Engine/EditorBlueprintResources/StandardMacros.IsValid` (`self.playerSaveGameRef`)
    (:`Is Valid`
      _)
    (:`Is Not Valid`
      (bind _returnvalue (`GameplayStatics.CreateSaveGameObject` "/Game/MCS/Blueprints/AllLevels/MCSPlayerSaveGame.MCSPlayerSaveGame_C"))
      (set `self.playerSaveGameRef` _returnvalue)))
  (bind _returnvalue_2 (`GameplayStatics.SaveGameToSlot` (`self.playerSaveGameRef`) (`self.PlayerProfileSave`)))
  (if (not _returnvalue_2)
    (`self.ShowErrorMessage` "Unable to save profile")))

(fn `TravelErrorToString`
  (params (failureType :type "ETravelFailure Enum"))
  (returns (outputString :type String))
  (return ""))