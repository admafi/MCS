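; Game mode for a two-player lightsaber duel that spawns fighters at PlayerStarts and makes later logins spectators.
; Once both join, it links them as enemies and pushes saber color, hit detection and recoil settings to them.
; Tick times each player's swing; on a clash, a sufficiently shorter swing wins and the loser gets a different recoil rate.
; It also applies stubbed flat damage and offers debug toggles and bot respawn.
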(event `ToggleTraceHits`
  ;[0.495 1 0.7074] Server Options
  (bind _output_get (set `/Game/MCS/Blueprints/MCSCharacter.ShowTraceHits` (not (`/Game/MCS/Blueprints/MCSCharacter.ShowTraceHits` (`self.Player_1`))) (`self.Player_1`)))
  (bind _output_get_2 (set `/Game/MCS/Blueprints/MCSCharacter.ShowTraceHits` _output_get (`self.Player_2`)))
  (`KismetSystemLibrary.PrintString` (`KismetStringLibrary.Concat_StrStr` "Show Hit Locations:  " (`KismetStringLibrary.Conv_BoolToString` _output_get_2))))

(event `SetTimeDilation`
  (params (`Dilation Amount` :type "Float (double-precision)"))
  ;[0.495 1 0.7074] Server Options
  (bind _output_get (set `self.TimeDilation` `Dilation Amount`))
  (`GameplayStatics.SetGlobalTimeDilation` _output_get))

(event `InitCombatPlayers`
  ;[1 1 1] Initialize the combat players. Most of these values will come from the player selects in a "lobby".  i.e. Saber color, etc.
  (`|ExecutionSequence`
    (:`then_0`
      ;;[1 1 1] Hide players untill ready
      (`self.SetActorHiddenInGame` (`self.Player_1`) false)
      (`self.SetActorHiddenInGame` (`self.Player_2`) false))
    (:`then_1`
      ;;[1 1 1] Combat player 1
      (`/Game/MCS/Blueprints/MCSCharacter.ChangeSaberColor` (`self.Player_1`) (`self.Player1SaberColor`))
      (bind _weapon (`self.GetPlayerWeapon` (`self.Player_1`)))
      (set `/Game/MCS/Blueprints/Lightsaber.HitDetectionType` (`self.HitDetectionType`) _weapon)
      (set `/Game/MCS/Blueprints/Lightsaber.NoCollisionWhenIdle` (`self.NoCollisionWhenIdle`) _weapon)
      (set `/Game/MCS/Blueprints/MCSCharacter.DefaultRecoilPlayRate` (`self.DefaultRecoilPlayRate`) (`self.Player_1`))
      (set `/Game/MCS/Blueprints/Lightsaber.ExcludedBones` (`self.ExcludedBones`) _weapon))
    (:`then_2`
      ;;[1 1 1] Combat Player 2
      (`/Game/MCS/Blueprints/MCSCharacter.ChangeSaberColor` (`self.Player_2`) (`self.Player2SaberColor`))
      (bind _weapon_2 (`self.GetPlayerWeapon` (`self.Player_2`)))
      (set `/Game/MCS/Blueprints/Lightsaber.HitDetectionType` (`self.HitDetectionType`) _weapon_2)
      (set `/Game/MCS/Blueprints/Lightsaber.NoCollisionWhenIdle` (`self.NoCollisionWhenIdle`) _weapon_2)
      (set `/Game/MCS/Blueprints/MCSCharacter.IsPracticeBot?` (`self.bUseBot`) (`self.Player_2`))
      (set `/Game/MCS/Blueprints/MCSCharacter.DefaultRecoilPlayRate` (`self.DefaultRecoilPlayRate`) (`self.Player_2`))
      (set `/Game/MCS/Blueprints/Lightsaber.ExcludedBones` (`self.ExcludedBones`) _weapon_2))
    (:`then_3`
      ;;[1 1 1] Notify clients that the server is ready
      (`/Game/MCS/Blueprints/MCSCharacter.ServerIsReady` (`self.Player_1`) (`self.Player1SaberColor`))
      (`/Game/MCS/Blueprints/MCSCharacter.ServerIsReady` (`self.Player_2`) (`self.Player2SaberColor`)))))

(event `DisplayPlayerSpeeds`
  (`KismetSystemLibrary.PrintString` (`KismetStringLibrary.Concat_StrStr` "PLAYER 1: " (`KismetStringLibrary.Conv_DoubleToString` (`CharacterMovementComponent.MaxWalkSpeed` (`Character.CharacterMovement` (`self.Player_1`)))) "  " "PLAYER 2: " (`KismetStringLibrary.Conv_DoubleToString` (`CharacterMovementComponent.MaxWalkSpeed` (`Character.CharacterMovement` (`self.Player_2`))))) true true (struct :`G` 0.66 :`B` 1.0 :`A` 1.0) 10.0))

(event `RespawnBot`
  (bind _player_1 (`self.Player_1`))
  (bind _player_2 (`self.Player_2`))
  ;[1 1 1] FOR TESTING: Reset/Respawn the practice bot player
  (`self.K2_DestroyActor` (`self.Player_2`))
  (`KismetSystemLibrary.Delay` 0.4)
  (bind _returnvalue (`|SpawnActorFromClass` "/Game/MCS/Blueprints/MCSCharacter.MCSCharacter_C" (`self.Player2Transform`) "Undefined" "OverrideRootScale" (`|GetArrayItem` (`self.CurrentPlayers`) 1)))
  (bind _output_get (set `self.Player_2` _returnvalue))
  (`Controller.Possess` (`|GetArrayItem` (`self.CurrentPlayers`) 1) _output_get)
  (`KismetSystemLibrary.Delay` 1.0)
  (`/Game/MCS/Blueprints/MCSCharacter.OnSetEnemyPlayer` _player_2 _player_2 (`self.Player_1`))
  (`/Game/MCS/Blueprints/MCSCharacter.OnSetEnemyPlayer` _player_1 _player_1 (`self.Player_2`))
  (`/Game/MCS/Blueprints/MCSCharacter.ChangeSaberColor` (`self.Player_2`) (`self.Player2SaberColor`))
  (bind _weapon (`self.GetPlayerWeapon` (`self.Player_2`)))
  (set `/Game/MCS/Blueprints/Lightsaber.HitDetectionType` (`self.HitDetectionType`) _weapon)
  (set `/Game/MCS/Blueprints/Lightsaber.NoCollisionWhenIdle` (`self.NoCollisionWhenIdle`) _weapon)
  (set `/Game/MCS/Blueprints/MCSCharacter.IsPracticeBot?` (`self.bUseBot`) (`self.Player_2`))
  (set `/Game/MCS/Blueprints/MCSCharacter.DefaultRecoilPlayRate` (`self.DefaultRecoilPlayRate`) (`self.Player_2`))
  (set `/Game/MCS/Blueprints/Lightsaber.ExcludedBones` (`self.ExcludedBones`) _weapon)
  (set `/Game/MCS/Blueprints/MCSCharacter.Health` 100.0 (`self.Player_2`))
  (set `/Game/MCS/Blueprints/MCSCharacter.Health` 100.0 (`self.Player_1`))
  (`/Game/MCS/Blueprints/MCSCharacter.ServerIsReady` (`self.Player_2`) (`self.Player2SaberColor`))
  (`KismetSystemLibrary.PrintString` "Spawned a bot.  Player health has been reset." true true (struct :`G` 0.66 :`B` 1.0 :`A` 1.0) 5.0))

(event `self.K2_PostLogin`
  (params (NewPlayer :type "PlayerController Object Reference"))
  (bind _player_1 (`self.Player_1`))
  (bind _player_2 (`self.Player_2`))
  ;[1 1 1] Spawn combat player
  (set `self.NewController` NewPlayer)
  (if (< (`KismetArrayLibrary.Array_Length` (`self.CurrentPlayers`)) 2)
    (`self.SpawnCombatPlayer` (`self.NewController`)) ; Once a player is spawned, he will be added to the currentPlayers array
    (if (== (`KismetArrayLibrary.Array_Length` (`self.CurrentPlayers`)) 2)
      (`KismetSystemLibrary.Delay` 1.0)
      (`/Game/MCS/Blueprints/MCSCharacter.OnSetEnemyPlayer` _player_1 _player_1 (`self.Player_2`))
      (`/Game/MCS/Blueprints/MCSCharacter.OnSetEnemyPlayer` _player_2 _player_2 (`self.Player_1`))
      (`KismetSystemLibrary.Delay` 1.0)
      (`self.InitCombatPlayers`))
    (else
      ;[1 1 1] Two combat players already spawned.  Spawn spectator(s)
      (`KismetSystemLibrary.Delay` 1.0)
      (bind _returnvalue (`|SpawnActorFromClass` "/Game/MCS/Blueprints/MCSSpectatorPawn.MCSSpectatorPawn_C" (`KismetMathLibrary.MakeTransform` (`self.SpectatorStartLocation`)) "Undefined" "OverrideRootScale"))
      (bind _output_get (set `self.NewSpectator` _returnvalue))
      (`Controller.Possess` (`self.NewController`) _output_get))))

(event `self.ReceiveBeginPlay`
  ;[1 1 1] Initialize spawn locations for combat players
  (`self.SetSpawnLocations`))

(event `self.HandleStartingNewPlayer`
  (params (NewPlayer :type "PlayerController Object Reference")))

(event `ApplyDamage`
  (params (hitResult :type "HitResult Structure") (CausedBy :type "/Game/MCS/Blueprints/MCSCharacter Object Reference"))
  ;[1 0.38 0.38] Calculate damage amount based on the hit information and game mode rules.
  (bind _output_get (set `self.hitResult` hitResult))
  (bind _damage (`self.CalculateDamage` _output_get))
  (bind (_bblockinghit _binitialoverlap _time _location _impactpoint _normal _impactnormal _physmat _hitactor) (`GameplayStatics.BreakHitResult` _output_get))
  (`GameplayStatics.ApplyPointDamage` _hitactor _damage _impactnormal (`self.hitResult`) null CausedBy "/Script/Engine.DamageType"))

(event `CycleHitDetectionType`
  ;[1 1 1] Cycle hit detection implementation for both combat players
  (switch `/Game/MCS/Blueprints/Enums/MCSHitDetectionType` (`self.HitDetectionType`)
    (:`NewEnumerator0`
      (set `self.HitDetectionType` "NewEnumerator1"))
    (:`NewEnumerator1`
      (set `self.HitDetectionType` "NewEnumerator2"))
    (:`NewEnumerator2`
      (set `self.HitDetectionType` "NewEnumerator0")))
  (bind _weapon (`self.GetPlayerWeapon` (`self.Player_1`)))
  (set `/Game/MCS/Blueprints/Lightsaber.HitDetectionType` (`self.HitDetectionType`) _weapon)
  (bind _weapon_2 (`self.GetPlayerWeapon` (`self.Player_2`)))
  (set `/Game/MCS/Blueprints/Lightsaber.HitDetectionType` (`self.HitDetectionType`) _weapon_2)
  (`KismetSystemLibrary.PrintString` (`KismetStringLibrary.Concat_StrStr` "Hit Detection changed to: " (`|GetEnumeratorNameAsString` (`self.HitDetectionType`)))))

(event `self.ReceiveTick`
  (params (DeltaSeconds :type "Float (single-precision)"))
  (bind _player_2 (`self.Player_2`))
  (bind _player_1 (`self.Player_1`))
  (set `self.DeltaSeconds` DeltaSeconds)
  (`/Engine/EditorBlueprintResources/StandardMacros.IsValid` (`self.Player_1`)
    (:`Is Valid`
      (`/Engine/EditorBlueprintResources/StandardMacros.IsValid` (`self.Player_2`)
        (:`Is Valid`
          (if (and (not (`/Game/MCS/Blueprints/MCSCharacter.IsDead?` (`self.Player_1`))) (not (`/Game/MCS/Blueprints/MCSCharacter.IsDead?` (`self.Player_2`))))
            (bind _weapon (`self.GetPlayerWeapon` (`self.Player_1`)))
            (bind _weapon_2 (`self.GetPlayerWeapon` (`self.Player_2`)))
            (set `self.DistanceBetweenWeapons` (`self.GetDistanceTo` _weapon _weapon_2))
            (set `self.DistanceBetweenPlayers` (`self.GetDistanceTo` (`self.Player_1`) (`self.Player_2`)))
            ;[1 1 1] Store values for both players swing times (attack time).  These values are used in the clash/block logic.
            (`|ExecutionSequence`
              (:`then_0`
                (if (`/Game/MCS/Blueprints/MCSCharacter.IsAttacking?` (`self.Player_1`))
                  (set `/Game/MCS/Blueprints/MCSCharacter.AttackTime` (+ (`/Game/MCS/Blueprints/MCSCharacter.AttackTime` _player_1) (`self.DeltaSeconds`)) _player_1)
                  (else
                    (set `/Game/MCS/Blueprints/MCSCharacter.AttackTime` 0.0 (`self.Player_1`)))))
              (:`then_1`
                (if (`/Game/MCS/Blueprints/MCSCharacter.IsAttacking?` (`self.Player_2`))
                  (bind _output_get (set `/Game/MCS/Blueprints/MCSCharacter.AttackTime` (+ (`/Game/MCS/Blueprints/MCSCharacter.AttackTime` _player_2) (`self.DeltaSeconds`)) _player_2))
                  (else
                    (bind _output_get_2 (set `/Game/MCS/Blueprints/MCSCharacter.AttackTime` 0.0 (`self.Player_2`)))))))))))))

(event `ResolveClash`
  ;[1 1 1] Clashing
  (set `self.ClashTime1` (`/Game/MCS/Blueprints/MCSCharacter.AttackTime` (`self.Player_1`)))
  (set `self.ClashTime2` (`/Game/MCS/Blueprints/MCSCharacter.AttackTime` (`self.Player_2`)))
  (bind (_playrate1 _playrate2) (`self.HandleClash`))
  (set `self.PlayRate1` _playrate1)
  (set `self.PlayRate2` _playrate2)
  (set `/Game/MCS/Blueprints/MCSCharacter.AttackTime` 0.0 (`self.Player_1`))
  (set `/Game/MCS/Blueprints/MCSCharacter.AttackTime` 0.0 (`self.Player_2`))
  (set `/Game/MCS/Blueprints/MCSCharacter.RecoilPlayRate` (`self.PlayRate1`) (`self.Player_1`))
  (set `/Game/MCS/Blueprints/MCSCharacter.RecoilPlayRate` (`self.PlayRate2`) (`self.Player_2`))
  (`|ExecutionSequence`
    (:`then_0`
      (`/Game/MCS/Blueprints/MCSCharacter.RecoilMulticast` (`self.Player_1`) (`self.PlayRate1`)))
    (:`then_1`
      (`/Game/MCS/Blueprints/MCSCharacter.RecoilMulticast` (`self.Player_2`) (`self.PlayRate2`)))))

(fn `CalculateDamage`
  (params (hitResult :type "HitResult Structure"))
  (returns (Damage :type "Float (double-precision)"))
  ;[1 1 1] STUB: Calculate damage here
  (return (`self.DefaultBaseDamage`)))

(fn `HandleClash`
  (returns (PlayRate1 :type "Float (double-precision)") (PlayRate2 :type "Float (double-precision)"))
  (bind _canclashstartingfromtime (`self.CanClashStartingFromTime`))
  (bind _defaultrecoilplayrate (`self.DefaultRecoilPlayRate`))
  (bind _defaultrecoilplayrate_2 (`self.DefaultRecoilPlayRate`))
  (if (or (<= (`self.ClashTime1`) _canclashstartingfromtime) (<= (`self.ClashTime2`) _canclashstartingfromtime))
    (return _defaultrecoilplayrate _defaultrecoilplayrate)
    (elif (>= (`KismetMathLibrary.Abs` (- (`self.ClashTime1`) (`self.ClashTime2`))) (`self.ClashTimeDifference`))
      (if (< (`self.ClashTime1`) (`self.ClashTime2`))
        (return (`self.DefaultRecoilPlayRate`) (`self.ClashLoserRecoilRate`))
        (else
          (return (`self.ClashLoserRecoilRate`) (`self.DefaultRecoilPlayRate`))))
      (else
        (return _defaultrecoilplayrate_2 _defaultrecoilplayrate_2)))))

(fn `PrintClashInfo`
  (locals (Player1_Weapon :type "/Game/MCS/Blueprints/Lightsaber Object Reference") (Player2_Weapon :type "/Game/MCS/Blueprints/Lightsaber Object Reference") (Velocity_1 :type "Float (double-precision)" :default 0.0) (Velocity_2 :type "Float (double-precision)"))
  (bind _player_1 (`self.Player_1`))
  (bind _player1_weapon (`local.Player1_Weapon`))
  (bind _player2_weapon (`local.Player2_Weapon`))
  (bind _player_2 (`self.Player_2`))
  (bind (_bladehitbladeresult_bblockinghit _bladehitbladeresult_binitialoverlap _bladehitbladeresult_time) (`GameplayStatics.BreakHitResult` (`/Game/MCS/Blueprints/MCSCharacter.BladeHitBladeResult` _player_1)))
  (bind (_bladehitbladeresult_bblockinghit_2 _bladehitbladeresult_binitialoverlap_2 _bladehitbladeresult_time_2) (`GameplayStatics.BreakHitResult` (`/Game/MCS/Blueprints/MCSCharacter.BladeHitBladeResult` _player_2)))
  (bind _weapon (`self.GetPlayerWeapon` (`self.Player_1`)))
  (set `local.Player1_Weapon` _weapon)
  (bind _weapon_2 (`self.GetPlayerWeapon` (`self.Player_2`)))
  (set `local.Player2_Weapon` _weapon_2)
  (bind _returnvalue (`PrimitiveComponent.GetPhysicsLinearVelocity` (`/Game/MCS/Blueprints/Lightsaber.Blade` (`local.Player1_Weapon`)) "None"))
  (set `local.Velocity_1` (`KismetMathLibrary.VSize` _returnvalue))
  (bind _returnvalue_2 (`PrimitiveComponent.GetPhysicsLinearVelocity` (`/Game/MCS/Blueprints/Lightsaber.Blade` (`local.Player2_Weapon`)) "None"))
  (set `local.Velocity_2` (`KismetMathLibrary.VSize` _returnvalue_2))
  (`KismetSystemLibrary.PrintString` (`KismetStringLibrary.Concat_StrStr` "Player 1 (AttackTime):  " (`KismetStringLibrary.Conv_DoubleToString` (`/Game/MCS/Blueprints/MCSCharacter.AttackTime` _player_1)) "    " "Hit Result Time:  " (`KismetStringLibrary.Conv_DoubleToString` _bladehitbladeresult_time) "    " "Velocity (stored):  " (`KismetStringLibrary.Conv_DoubleToString` (`KismetMathLibrary.VSize` (`/Game/MCS/Blueprints/Lightsaber.LinearVelocityAtPoint` _player1_weapon))) "    " "Linear Velocity (stored):  " (`KismetStringLibrary.Conv_VectorToString` (`/Game/MCS/Blueprints/Lightsaber.LinearVelocity` _player1_weapon)) "    " "Linear Velocity at Point (stored):  " (`KismetStringLibrary.Conv_VectorToString` (`/Game/MCS/Blueprints/Lightsaber.LinearVelocityAtPoint` _player1_weapon)) "    " "Velocity (RT): " (`KismetStringLibrary.Conv_DoubleToString` (`local.Velocity_1`))) true true (struct :`R` 0.141904 :`G` 0.526455 :`B` 1.0 :`A` 1.0) 2.0)
  (`KismetSystemLibrary.PrintString` (`KismetStringLibrary.Concat_StrStr` "Player 2 (AttackTime):  " (`KismetStringLibrary.Conv_DoubleToString` (`/Game/MCS/Blueprints/MCSCharacter.AttackTime` _player_2)) "    " "Hit Result Time:  " (`KismetStringLibrary.Conv_DoubleToString` _bladehitbladeresult_time_2) "    " "Velocity (stored):  " (`KismetStringLibrary.Conv_DoubleToString` (`KismetMathLibrary.VSize` (`/Game/MCS/Blueprints/Lightsaber.LinearVelocityAtPoint` _player2_weapon))) "    " "Linear Velocity (stored):  " (`KismetStringLibrary.Conv_VectorToString` (`/Game/MCS/Blueprints/Lightsaber.LinearVelocity` _player2_weapon)) "    " "Linear Velocity at Point (stored):  " (`KismetStringLibrary.Conv_VectorToString` (`/Game/MCS/Blueprints/Lightsaber.LinearVelocityAtPoint` _player2_weapon)) "    " "Velocity (RT): " (`KismetStringLibrary.Conv_DoubleToString` (`local.Velocity_2`))) true true (struct :`R` 1.0 :`G` 0.794904 :`A` 1.0) 2.0))

(fn `SetSpawnLocations`
  (locals (currentIndex :type Integer) (currentPlayerStart :type "PlayerStart Object Reference"))
  (bind _outactors (`GameplayStatics.GetAllActorsOfClass` "/Script/Engine.PlayerStart"))
  (bind _output_get (set `self.PlayerStartArray` _outactors))
  (if (> (`KismetArrayLibrary.Array_Length` _output_get) 0)
    (for (_array_element _array_index) (`self.PlayerStartArray`)
      (set `local.currentPlayerStart` _array_element)
      (bind _output_get_2 (set `local.currentIndex` _array_index))
      (if (<= _output_get_2 1)
        (if (== (`local.currentIndex`) 0)
          (set `self.Player1Transform` (`self.GetTransform` (`local.currentPlayerStart`)))
          (elif (== (`local.currentIndex`) 1)
            (set `self.Player2Transform` (`self.GetTransform` (`local.currentPlayerStart`)))))
        (else
          (break))))))

(fn `SpawnCombatPlayer`
  (params (Player :type "PlayerController Object Reference"))
  (locals (currentIndex :type Integer) (combatPlayer :type "PlayerController Object Reference"))
  (set `local.combatPlayer` Player)
  (if (< (`KismetArrayLibrary.Array_Length` (`self.CurrentPlayers`)) 1)
    (bind _returnvalue (`|SpawnActorFromClass` "/Game/MCS/Blueprints/MCSCharacter.MCSCharacter_C" (`self.Player1Transform`) "Undefined" "OverrideRootScale" (`local.combatPlayer`)))
    (bind _output_get (set `self.Player_1` _returnvalue))
    (`Controller.Possess` (`local.combatPlayer`) _output_get)
    (`KismetArrayLibrary.Array_Add` (`self.CurrentPlayers`) (`local.combatPlayer`))
    (else
      (bind _returnvalue_2 (`|SpawnActorFromClass` "/Game/MCS/Blueprints/MCSCharacter.MCSCharacter_C" (`self.Player2Transform`) "Undefined" "OverrideRootScale" (`local.combatPlayer`)))
      (bind _output_get_2 (set `self.Player_2` _returnvalue_2))
      (`Controller.Possess` (`local.combatPlayer`) _output_get_2)
      (`KismetArrayLibrary.Array_Add` (`self.CurrentPlayers`) (`local.combatPlayer`)))))

(fn `UserConstructionScript`)